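; BP_Health tracks a Health value and provides functions to raise and lower it.
; IncreaseHealth adds an amount clamped between zero and MaxHealth, while DecreaseHealth subtracts damage without clamping.
; Both functions call UpdatedHealth after each change, and DecreaseHealth also calls Death whenever Health is at or below zero.
; The event graph holds only disabled BeginPlay and Tick placeholders, so all logic runs through these two functions.
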(event EventBeginPlay)

(event EventTick
  (params (DeltaSeconds :type Float%20%28single-precision%29)))

(fn IncreaseHealth
  (params (HealthAmount :type Float%20%28double-precision%29))
  (Variables|Default|SetHealth (Math|Float|Clamp(Float) (+ (Variables|Default|GetHealth) HealthAmount) 0.0 (Variables|Default|GetMaxHealth)))
  (Default|CallUpdatedHealth))

(fn DecreaseHealth
  (params (Damage :type Float%20%28double-precision%29))
  (Variables|Default|SetHealth (- (Variables|Default|GetHealth) Damage))
  (Default|CallUpdatedHealth)
  (if (<= (Variables|Default|GetHealth) 0.0)
    (Default|CallDeath)))