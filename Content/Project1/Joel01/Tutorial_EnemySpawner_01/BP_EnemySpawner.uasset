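; Enemy spawner that keeps a set number of AI enemies of a chosen type alive, topping them up on Tick.
; At BeginPlay it filters data table rows by enemy type, then spawns BP_SpawnedEnemy pawns from randomly picked rows.
; Each spawn receives its row as SpawnInfo, initializes its RPG sheet from it and binds a death event on its DamageBrain.
; OnMobDeath removes the mob from the tracked list, freeing a slot for respawn.
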(event Custom|OnMobDeath
  (params (deadMob :type Actor%20Object%20Reference))
  (bind _returnvalue (Utilities|Array|RemoveItem (Variables|Default|GetspawnedEnemies) deadMob))
  (Development|PrintString (Utilities|String|Append "Mob died: " (Utilities|GetObjectName deadMob) ", Removed: " (Utilities|String|ToString(Boolean) _returnvalue))))

(event EventBeginPlay
  (Utilities|PopulateArrayfromTable (Variables|Default|GettypeToSpawn) (Variables|Default|GetenemyArray))
  (CallFunction|SpawnRemaning))

(event EventTick
  (params (DeltaSeconds :type Float%20%28single-precision%29))
  (if (< (Utilities|Array|Length (Variables|Default|GetspawnedEnemies)) (Variables|Default|Getamount))
    (CallFunction|SpawnRemaning)))

(fn ConstructionScript)

(fn SpawnRemaning
  (for _index (range (Utilities|Array|Length (Variables|Default|GetspawnedEnemies)) (- (Variables|Default|Getamount) 1))
    (Utilities|SpawnRandomEnemy)))

(fn OnSpawnedMob
  (params (newMob :type Pawn%20Object%20Reference) (spawnInfo :type S%20Enemy%20Spawn%20Info%20Structure) (index :type Integer))
  (bind _returnvalue (Actor|GetComponentbyClass newMob "/Game/Project1/Joel01/RPGSheet/RPGSheetBrain.RPGSheetBrain_C"))
  (bind _asbp_spawned_enemy (Utilities|Casting|CastToBP_SpawnedEnemy newMob))
  (Variables|/Game/Project1/Joel01/Tutorial_AI_01/BP_SpawnedEnemy.BP_SpawnedEnemy_C|SetspawnInfo _asbp_spawned_enemy spawnInfo)
  (EventDispatchers|BindEventtoOnDeathDetailed (Variables|/Game/Project1/Joel01/Tutorial_AI_01/BP_SpawnedEnemy.BP_SpawnedEnemy_C|GetDamageBrain _asbp_spawned_enemy) (EventDispatchers|CreateEvent :!event Custom|OnMobDeath))
  ;[0.63 0.15 0.15 0.5] Hacky way of loading the sheet from a data table
  (Utilities|IsValid _returnvalue
    (:Is%20Valid
      (Default|InitializeSheetfrom _returnvalue (.rpgSheet (Utilities|Struct|BreakS_EnemySpawnInfo spawnInfo))))
    (:Is%20Not%20Valid
      (Development|PrintString "Sheet not valid"))))