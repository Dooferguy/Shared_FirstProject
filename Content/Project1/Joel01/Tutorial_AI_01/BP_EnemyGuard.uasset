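; Enemy guard that patrols randomly chosen tagged actors, chases the player and can be damaged and killed.
; AIMoveTo drives a looping patrol with pauses; perception updates switch to a faster chase of the player, and forgetting the player slows it back into patrol.
; DamageBrain handles health behind damage, heal and health functions, with a health widget created on BeginPlay.
; On death it enables mesh physics, disables sight and stops further patrol loops.
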(event OnTargetPerceptionUpdated(AIPerception)
  (params (Actor :type Actor%20Object%20Reference) (Stimulus :type AI%20Stimulus%20Structure))
  (if (not (Variables|Default|GetisDead))
    (bind _asbp_joel_player (Utilities|Casting|CastToBP_Joel_Player Actor))
    (Variables|/Script/Engine.CharacterMovementComponent|SetMaxWalkSpeed (Variables|Character|GetCharacterMovement) 5e+02)
    (AI|AIMoveTo self "0, 0, 0" _asbp_joel_player 5.0 false)))

(event OnTargetPerceptionForgotten(AIPerception)
  (params (Actor :type Actor%20Object%20Reference))
  (Utilities|Casting|CastToBP_Joel_Player Actor)
  (Variables|/Script/Engine.CharacterMovementComponent|SetMaxWalkSpeed (Variables|Character|GetCharacterMovement) 3e+02)
  (if (not (Variables|Default|GetisDead)) :!label _label
    (bind _outactors (Actor|GetAllActorswithTag (Variables|Default|GetTag)))
    (AI|AIMoveTo self "0, 0, 0" (.OutItem (Utilities|Array|Random _outactors)) 5.0 false
      (:OnSuccess
        (Utilities|FlowControl|Delay 2.0)
        (goto _label)))))

(event OnDeath(DamageBrain)
  (bind _mesh (Variables|Character|GetMesh))
  ;[0.15 0.15 0.15 0.5] SimpleDamageable
  (Physics|SetSimulatePhysics _mesh true)
  (Collision|SetCollisionEnabled _mesh "QueryAndPhysics")
  (Class|AIPerceptionComponent|SetSenseEnabled (Variables|Default|GetAIPerception) "/Script/AIModule.AISense_Sight" false)
  (Variables|Default|SetisDead true))

(event Custom|OnTargetPerceptionForgotten_Event
  (params (Actor :type Actor%20Object%20Reference)))

(event EventBeginPlay
  (bind _returnvalue (UserInterface|CreateWidget "/Game/Project1/Tutorial2/SimpleHealthWidget.SimpleHealthWidget_C" 0 self))
  (UserInterface|SetWidget (Variables|Default|GetWidget) _returnvalue)
  (EventDispatchers|AssignOnTargetPerceptionForgotten (Variables|Default|GetAIPerception) (delegate Custom|OnTargetPerceptionForgotten_Event))
  (bind _outactors (Actor|GetAllActorswithTag (Variables|Default|GetTag) :!label _label))
  (AI|AIMoveTo self "0, 0, 0" (.OutItem (Utilities|Array|Random _outactors)) 5.0 false
    (:OnSuccess
      (Utilities|FlowControl|Delay 2.0)
      (if (not (Variables|Default|GetisDead))
        (goto _label)))))

(fn ConstructionScript)

(fn DamageTaken
  (params (DamageInfo :type Damage%20Info%20Structure))
  (bind _wasdamaged (Default|Damage (Variables|Default|GetDamageBrain) DamageInfo))
  (return _wasdamaged))

(fn GetCurrentHealth
  (bind _health (Default|GetHealth (Variables|Default|GetDamageBrain)))
  (return _health))

(fn GetMaxHealth
  (bind _maxhealth (Default|GetHealthMax (Variables|Default|GetDamageBrain)))
  (return _maxhealth))

(fn HealSelf
  (params (AmountHealed :type Float%20%28double-precision%29))
  (bind _updatedhealth (Default|Heal (Variables|Default|GetDamageBrain) AmountHealed))
  (return _updatedhealth))