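; Spawned enemy character that patrols between random tagged actors, chases the player on perception and drops loot on death.
; AI perception switches between faster chase and patrol, while a looping timer sphere-traces ahead to deal damage.
; DamageBrain backs the damage interface and health widget; death ragdolls the mesh and spawns loot-table items at the player's transform.
; SpawnInfo sets mesh and animation after a short delay that works around spawned-AI pathing.
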(event OnTargetPerceptionUpdated(AIPerception)
  (params (Actor :type Actor%20Object%20Reference) (Stimulus :type AI%20Stimulus%20Structure))
  ;[0.15 0.15 0.15 0.5] Tutorial Content + Cleanup (Event call)
  (if (not (Variables|Default|GetisDead))
    (bind _asbp_joel_player (Utilities|Casting|CastToBP_Joel_Player Actor))
    (Variables|/Script/Engine.CharacterMovementComponent|SetMaxWalkSpeed (Variables|Character|GetCharacterMovement) 5e+02)
    (AI|AIMoveTo self "0, 0, 0" _asbp_joel_player 5.0 false)))

(event OnTargetPerceptionForgotten(AIPerception)
  (params (Actor :type Actor%20Object%20Reference))
  ;[0.15 0.15 0.15 0.5] Tutorial Content + Cleanup (Event call)
  (Utilities|Casting|CastToBP_Joel_Player Actor)
  (Variables|/Script/Engine.CharacterMovementComponent|SetMaxWalkSpeed (Variables|Character|GetCharacterMovement) 3e+02)
  (CallFunction|LookforPatrolPoint))

(event OnDeath(DamageBrain)
  (bind _mesh (Variables|Character|GetMesh))
  ;[0.15 0.15 0.15 0.5] SimpleDamageable
  (Physics|SetSimulatePhysics _mesh true)
  (Collision|SetCollisionEnabled _mesh "QueryAndPhysics")
  (Class|AIPerceptionComponent|SetSenseEnabled (Variables|Default|GetAIPerception) "/Script/AIModule.AISense_Sight" false)
  (Variables|Default|SetisDead true)
  (Collision|SetCollisionEnabled (Variables|Collision|GetCapsuleComponent) "NoCollision")
  (bind _rowhandle (Default|GetRowfromTable (Variables|Default|GetLootTableSystem)))
  ;[0.15 0.15 0.15 0.5] Drop Loot
  (Game|SpawnActorfromClass :Class "/Game/Project1/Joel01/Items/BP_LootItem.BP_LootItem_C" :SpawnTransform (Transformation|GetActorTransform (Game|GetPlayerCharacter 0)) :CollisionHandlingOverride "Undefined" :TransformScaleMethod "MultiplyWithRoot" :dataSource _rowhandle :Instigator 0))

(event Custom|OnTargetPerceptionForgotten_Event
  (params (Actor :type Actor%20Object%20Reference)))

(event Custom|LookForPatrolPoint
  ;[0.15 0.15 0.15 0.5] Tutorial Content + Cleanup (Event call)
  (if (not (Variables|Default|GetisDead))
    (bind _outactors (Actor|GetAllActorswithTag (Variables|Default|GetTag)))
    (bind _movementresult (AI|AIMoveTo self "0, 0, 0" (.OutItem (Utilities|Array|Random _outactors)) 5.0 false)
      (:OnSuccess
        (Utilities|FlowControl|Delay 2.0))
      (:OnFail
        (Development|PrintString "Moveto failed")))
    (CallFunction|LookforPatrolPoint)))

(event Custom|Attack
  (bind _returnvalue (Default|IsDead (Variables|Default|GetDamageBrain)))
  (if (not _returnvalue)
    (bind (_location _hitactor _washit) (Utilities|CastHit))
    (if _washit
      (Utilities|OnHit _location _hitactor))))

(event EventBeginPlay
  (Default|InitializewithTarget (Variables|Default|GetSimpleHealthComponent) self (Variables|Default|GetWidget))
  (Utilities|Time|SetTimerbyEvent (delegate Custom|Attack) 2.0 true)
  (EventDispatchers|AssignOnTargetPerceptionForgotten (Variables|Default|GetAIPerception) (delegate Custom|OnTargetPerceptionForgotten_Event))
  ;[0.15 0.15 0.15 0.5] Hack: Fixes spawned AI not pathing
  (Utilities|FlowControl|Delay 0.2)
  (CallFunction|LookforPatrolPoint)
  (Utilities|SetMeshfromSpawnInfo))

(fn ConstructionScript)

(fn DamageTaken
  (params (DamageInfo :type Damage%20Info%20Structure))
  (bind _wasdamaged (Default|Damage (Variables|Default|GetDamageBrain) DamageInfo))
  (return _wasdamaged))

(fn GetCurrentHealth
  (bind _health (Default|GetHealth (Variables|Default|GetDamageBrain)))
  (return _health))

(fn GetExperienceReward
  (bind _result (Default|GetStat (Variables|Default|GetRPGSheetBrain) "NewEnumerator2"))
  (return (.currentvalue _result)))

(fn GetMaxHealth
  (bind _maxhealth (Default|GetHealthMax (Variables|Default|GetDamageBrain)))
  (return _maxhealth))

(fn HealSelf
  (params (AmountHealed :type Float%20%28double-precision%29))
  (bind _updatedhealth (Default|Heal (Variables|Default|GetDamageBrain) AmountHealed))
  (return _updatedhealth))