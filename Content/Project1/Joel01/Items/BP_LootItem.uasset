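; BP_LootItem is a loot item actor that shows the mesh of its item data on a physics-simulated static mesh.
; The construction script looks up the DataSource's data table row, stores it as Item and applies its mesh.
; SetItem replaces the item and mesh directly, while SetDataSource stores a new row handle and refreshes Item without updating the mesh.
; BeginPlay and SetItem print debug messages.
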(event EventBeginPlay
  (Development|PrintString "Begin play for spawned item"))

(fn ConstructionScript
  (bind _item (Utilities|SetItemfromDataSource))
  (Utilities|SetMesh (Variables|Default|GetStaticMesh) (.mesh _item)))

(fn SetItem
  (params (item :type S%20Item%20Structure%20Structure))
  (Development|PrintString "Set Item called")
  (bind _output_get (Variables|Default|SetItem item))
  (Utilities|SetMesh (Variables|Default|GetStaticMesh) (.mesh _output_get)))

(fn SetDataSource
  (params (dataSource :type Data%20Table%20Row%20Handle%20Structure))
  (Variables|Default|SetdataSource dataSource)
  (Utilities|SetItemfromDataSource))