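; Actor component that manages health, damage and death, with heal and take-damage functions.
; A CanBeDamaged macro routes each hit to blocked, damage or none using death, invincibility and block states, which damage-info flags can bypass.
; Event dispatchers announce blocks with parry eligibility, death, and damage responses when interruptible or forced.
; TakeDamage returns true only on death or a triggered response; Heal clamps to max health while alive.
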(event EventBeginPlay)

(event EventTick
  (params (DeltaSeconds :type Float%20%28single-precision%29)))

(fn Heal
  (params (Amount :type Float%20%28double-precision%29))
  (if (not (Variables|Default|GetDeath))
    (bind _output_get (Variables|Default|SetHealth (Math|Float|Clamp(Float) (+ Amount (Variables|Default|GetHealth)) 0.0 (Variables|Default|GetMaxhealth))))
    (return _output_get)))

(fn TakeDamage
  (params (DamageInfo :type Damage%20Info%20Structure))
  (bind (_damageamount _damagetype _damageresponse _damageinvincibleframe _canbeblocked _canbeparried _forceinterupt) (Utilities|Struct|BreakDamage_Info DamageInfo))
  (Utilities|CanbeDamaged _damageinvincibleframe _canbeblocked
    (:BlockedDamage
      (Default|CallOnBlocked _canbeparried)
      (return false))
    (:DoDamage
      (bind _output_get (Variables|Default|SetHealth (- (Variables|Default|GetHealth) _damageamount)))
      (if (<= _output_get 0.0)
        (Variables|Default|SetDeath true)
        (Default|CallOnDeath)
        (return true)
        (elif (or (Variables|Default|GetInteruptted) _forceinterupt)
          (Default|CallOnDamageResponse _damageresponse)
          (return true))))
    (:NoDamage
      (return false))))